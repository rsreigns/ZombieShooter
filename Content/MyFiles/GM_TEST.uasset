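; GM_TEST, apparently a test game mode, periodically spawns enemy AI during play.
; A looping timer started on BeginPlay fires SpawnAI, which randomly picks BP_BaseEnemyCharacter or BP_Crawler while their combined count stays under a cap.
; Spawns use a random reachable navmesh point around the player's negated, scaled forward vector.
; That vector is not added to the player's location, so the search centers near world origin.
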(event `self.ReceiveBeginPlay`
  (bind _returnvalue (`KismetSystemLibrary.K2_SetTimerDelegate` (delegate `SpawnAI`) 4.0 true))
  (set `self.TimerHandle` _returnvalue))

(event `SpawnAI`
  (set `self.RandomValue` (`KismetMathLibrary.RandomBool`))
  (bind _outactors (`GameplayStatics.GetAllActorsOfClass` "/Game/MyFiles/AI/BP_BaseEnemyCharacter.BP_BaseEnemyCharacter_C"))
  (bind _outactors_2 (`GameplayStatics.GetAllActorsOfClass` "/Game/MyFiles/AI/BP_Crawler.BP_Crawler_C"))
  (if (< (+ (`KismetArrayLibrary.Array_Length` _outactors_2) (`KismetArrayLibrary.Array_Length` _outactors)) 40)
    (`|SpawnActorFromClass` (select `bool` (`self.RandomValue`) :`false` "/Game/MyFiles/AI/BP_Crawler.BP_Crawler_C" :`true` "/Game/MyFiles/AI/BP_BaseEnemyCharacter.BP_BaseEnemyCharacter_C" :!type "Actor Class Reference") (`KismetMathLibrary.MakeTransform` (`NavigationSystemV1.K2_GetRandomReachablePointInRadius` (* (`self.GetActorForwardVector` (`GameplayStatics.GetPlayerPawn` 0)) -700.0) 1500.0 null null)) "AdjustIfPossibleButAlwaysSpawn" "MultiplyWithRoot" null null)))

(fn `UserConstructionScript`)