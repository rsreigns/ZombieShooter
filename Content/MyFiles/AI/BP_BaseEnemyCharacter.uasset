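; BP_BaseEnemyCharacter is the base enemy character, with a random walk speed set at BeginPlay.
; A sphere overlap stores the player and starts a looping three-second timer that plays an attack montage.
; When the player leaves the sphere, the stored reference and timer are cleared.
; An ApplyDamage call exists but is unconnected, so this graph's attack only plays animation.
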(event `self.ReceiveBeginPlay`
  (set `CharacterMovementComponent.MaxWalkSpeed` (`KismetMathLibrary.Conv_IntToDouble` (`KismetMathLibrary.RandomIntegerInRange` 40 120)) (`self.CharacterMovement`)))

(event `Startattack`
  (`|PlayMontage` (`self.Mesh`) "/Game/MyFiles/Animation/Enemy/Montages/AM_Attack2.AM_Attack2"))

(event `self.Sphere.OnComponentBeginOverlap`
  (params (OverlappedComponent :type "PrimitiveComponent Object Reference") (OtherActor :type "Actor Object Reference") (OtherComp :type "PrimitiveComponent Object Reference") (OtherBodyIndex :type Integer) (bFromSweep :type Boolean) (SweepResult :type "HitResult Structure (by ref)"))
  (`/Engine/EditorBlueprintResources/StandardMacros.IsValid` (`self.Player`)
    (:`Is Not Valid`
      (bind _asbp_my_character (cast `/Game/MyFiles/Pawns/BP_MyCharacter` OtherActor))
      (set `self.Player` _asbp_my_character)
      (bind _returnvalue (`KismetSystemLibrary.K2_SetTimerDelegate` (delegate `Startattack`) 3.0 true))
      (set `self.AttackTimerHandle` _returnvalue))))

(event `self.Sphere.OnComponentEndOverlap`
  (params (OverlappedComponent :type "PrimitiveComponent Object Reference") (OtherActor :type "Actor Object Reference") (OtherComp :type "PrimitiveComponent Object Reference") (OtherBodyIndex :type Integer))
  (cast `/Game/MyFiles/Pawns/BP_MyCharacter` OtherActor)
  (set `self.Player` null)
  (`KismetSystemLibrary.K2_ClearAndInvalidateTimerHandle` (`self.AttackTimerHandle`)))

(fn `UserConstructionScript`)